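; BP_PersonajeVM is a player character in the 2D folder, driven by Enhanced Input.
; BeginPlay adds its mapping context, and input actions handle forward-axis movement, yaw look and jumping.
; Movement also has a control-rotation step meant to follow a float comparison, but it compares constant zero to zero, so neither connected branch runs, and both would set zero rotation anyway.
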(event Input|EnhancedActionEvents|EnhancedInputActionIA_MirarVM
  (params (ActionValue :type Float%20%28double-precision%29) (ElapsedSeconds :type Float%20%28double-precision%29) (TriggeredSeconds :type Float%20%28double-precision%29) (InputAction :type Input%20Action%20Object%20Reference :default "/Game/2D/Blueprints/ImputAction/IA_MirarVM.IA_MirarVM"))
  (Pawn|Input|AddControllerYawInput ActionValue))

(event Input|EnhancedActionEvents|EnhancedInputActionIA_MovimientioVM
  (params (ActionValue :type Float%20%28double-precision%29) (ElapsedSeconds :type Float%20%28double-precision%29) (TriggeredSeconds :type Float%20%28double-precision%29) (InputAction :type Input%20Action%20Object%20Reference :default "/Game/2D/Blueprints/ImputAction/IA_MovimientioVM.IA_MovimientioVM"))
  (bind _returnvalue (Pawn|GetController))
  (Pawn|Input|AddMovementInput (* (Transformation|GetActorForwardVector) ActionValue) 1.0 false)
  (Math|Float|CompareFloat 0.0 0.0
    (:>
      (Pawn|SetControlRotation _returnvalue (Math|Rotator|MakeRotator 0.0 0.0 0.0)))
    (:<
      (Pawn|SetControlRotation _returnvalue (Math|Rotator|MakeRotator 0.0 0.0 0.0)))))

(event Input|EnhancedActionEvents|EnhancedInputActionIA_SaltarVM
  (params (ActionValue :type Float%20%28double-precision%29) (ElapsedSeconds :type Float%20%28double-precision%29) (TriggeredSeconds :type Float%20%28double-precision%29) (InputAction :type Input%20Action%20Object%20Reference :default "/Game/2D/Blueprints/ImputAction/IA_SaltarVM.IA_SaltarVM"))
  (:Started
    (Character|Jump))
  (:Completed
    (Character|StopJumping)))

(event EventBeginPlay
  (bind _asplayer_controller (Utilities|Casting|CastToPlayerController (Pawn|GetController)))
  (Input|AddMappingContext (PlayerController|LocalPlayerSubsystems|GetEnhancedInputLocalPlayerSubsystem _asplayer_controller) "/Game/2D/Blueprints/MapingContext/MC_PersonajeImputVM.MC_PersonajeImputVM" 0 "(bIgnoreAllPressedKeysUntilRelease=True,bForceImmediately=False,bNotifyUserSettings=False)"))

(fn ConstructionScript)